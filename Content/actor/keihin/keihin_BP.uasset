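; Prize actor (keihin) for a crane game that gets carried by the crane and then dropped.
; Any overlap rotates it and, after a delay, plays a timeline that snaps it to Crean_BP's location while axis comparisons against the crane's goal hold.
; Overlapping a "DownPoint"-tagged actor sets KeihinDown after a delay, stopping the follow.
; Tick then moves it by KeihinDownVector from its Box position each frame.
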(event EventTick
  (params (DeltaSeconds :type Float%20%28single-precision%29))
  (bind _returnvalue (Transformation|GetActorLocation))
  ;[1 1 1] ゴールについたら景品を落とす処理
  (Utilities|FlowControl|Sequence
    (:then_0
      (if (Variables|Default|GetKeihinDown)
        (Transformation|SetActorTransform (Math|Transform|MakeTransform (+ (Transformation|GetWorldLocation (Variables|Default|GetBox)) (Variables|Default|GetKeihin_Down_Vector) ""))) ; 景品を落とすポイントについた時処理
      ))
    (:then_1
      (Variables|Default|SetNow_Location_X (.x _returnvalue))
      (Variables|Default|SetNow_Location_Y (.y _returnvalue))
      (Variables|Default|SetNow_Location_Z (.z _returnvalue)))))

(event EventBeginPlay
  ;[1 1 1] widget作成
  (Utilities|FlowControl|Sequence
    (:then_0
      (bind _returnvalue (Actor|GetActorOfClass "/Game/actor/Character/Crean_BP.Crean_BP_C"))
      (Variables|Default|SetCrean_BP _returnvalue)
      (bind _returnvalue_2 (Actor|GetActorOfClass "/Game/actor/Goal/Keihin_downpoint_Blueprint.Keihin_downpoint_Blueprint_C"))
      (Variables|Default|Setkeihin_Down_BP _returnvalue_2)
      (Variables|Default|SetKeihinDown false))))

(event Collision|EventActorBeginOverlap
  (params (OtherActor :type Actor%20Object%20Reference))
  (bind _crean_bp (Variables|Default|GetCrean_BP))
  ;[1 1 1] craneについていく処理
  (Utilities|FlowControl|Sequence
    (:then_0
      (Transformation|SetActorTransform (Math|Transform|MakeTransform (Transformation|GetActorLocation) "0.000000,90.000000,0.000000" (Transformation|GetActorScale3D)))
      (Utilities|FlowControl|Delay 2.0)
      (Timeline|crean_carrytime Play
        (:Update
          (if (not (Variables|Default|GetKeihinDown))
            (Utilities|FlowControl|Sequence
              (:then_0
                (if (>= (Variables|Default|GetNow_Location_X) (Variables|/Game/actor/Character/Crean_BP.Crean_BP_C|GetGoalLocation_X _crean_bp))
                  (Transformation|SetActorTransform (Math|Transform|MakeTransform (Transformation|GetActorLocation _crean_bp) "0.000000,90.000000,0.000000" (Transformation|GetActorScale3D)) :!label _label)))
              (:then_1
                (if (>= (Variables|Default|GetNow_Location_Y) (Variables|/Game/actor/Character/Crean_BP.Crean_BP_C|GetGoalLocation_Y _crean_bp))
                  (goto _label)))
              (:then_2
                (if (<= (Variables|Default|GetNow_Location_Z) (Variables|/Game/actor/Character/Crean_BP.Crean_BP_C|GetGoalLocation_Z _crean_bp))
                  (goto _label))))))))
    (:then_1
      (if (Actor|ActorHasTag OtherActor "DownPoint")
        ;[1 1 1] ゴールについたら景品を落とす処理
        (Utilities|FlowControl|Delay 1.0)
        (Variables|Default|SetKeihinDown true)))))

(fn ConstructionScript)