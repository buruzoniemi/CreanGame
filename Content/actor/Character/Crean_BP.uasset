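; Player-controlled crane-game claw that moves horizontally, drops on the shift action and returns to its start point.
; Tick opens the arms, lowers the claw and projects a fake shadow via a downward trace into a dynamic material.
; Prize or floor overlaps trigger timelines that close the arms, step back along Z, Y, then X, and reopen.
; Wall tags nudge it back, BlockAction_BP overlaps block dropping, and a countdown sets TimeDown.
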(event OnComponentBeginOverlap(BlockDetection)
  (params (OverlappedComponent :type Primitive%20Component%20Object%20Reference) (OtherActor :type Actor%20Object%20Reference) (OtherComp :type Primitive%20Component%20Object%20Reference) (OtherBodyIndex :type Integer) (bFromSweep :type Boolean) (SweepResult :type Hit%20Result%20Structure%20%28by%20ref%29))
  ;[1 1 1] 出口の上にいるときに、クレーン下げらないように
  (Utilities|Casting|CastToBlockAction_BP OtherActor)
  (Variables|Default|SetBlockGrab true))

(event OnComponentEndOverlap(BlockDetection)
  (params (OverlappedComponent :type Primitive%20Component%20Object%20Reference) (OtherActor :type Actor%20Object%20Reference) (OtherComp :type Primitive%20Component%20Object%20Reference) (OtherBodyIndex :type Integer))
  ;[1 1 1] 出口の上にいるときに、クレーン下げらないように
  (Utilities|Casting|CastToBlockAction_BP OtherActor)
  (Variables|Default|SetBlockGrab false))

(event Custom|SpawnShadow
  ;[1 1 1] 丸影の処理
  (bind _outhit (Collision|LineTraceByChannel (+ (Transformation|GetActorLocation) "0.000000,0.000000,10.000000") (- (Transformation|GetActorLocation) "0.000000,0.000000,10000.000000") "TraceTypeQuery2" false 0 "None"))
  (Rendering|Material|SetScalarParameterValue (Variables|Default|GetShadowInstance) "GroundHeight" (.z (.Location (Collision|BreakHitResult _outhit))) :!class /Script/Engine.MaterialInstanceDynamic))

(event EventTick
  (params (DeltaSeconds :type Float%20%28single-precision%29))
  (bind _returnvalue (Transformation|GetActorLocation))
  ;[1 1 1] 下に動く
  (CallFunction|SpawnShadow)
  (Utilities|FlowControl|Sequence
    (:then_0
      ;[1 1 1] 時間の処理
      (if (> (Variables|Default|GetMax_Time_float) (Variables|Default|Getend_Time))
        (Variables|Default|SetDelta_Time_float DeltaSeconds)
        (Variables|Default|SetMax_Time_float (- (Variables|Default|GetMax_Time_float) (Variables|Default|GetDelta_Time_float)))))
    (:then_1
      (if (Variables|Default|GetCrean_down)
        (Utilities|FlowControl|Sequence
          (:then_0
            (if (> (Variables|Default|GetNow_R_arm_rotationY) (Variables|Default|GetMax_R_arm_rotationY))
              (Pawn|Input|AddMovementInput (Math|Vector|GetUpVector "0, 0, 0") -0.5 false) ; ScaleValue分、下に下がる。
              (Input|DisableInput 0)
              (else
                (Transformation|SetRelativeTransform (Variables|Default|GetR_arm) (Math|Transform|MakeTransform "270.000000,0.000000,-110.000000" (Math|Rotator|MakeRotator 0.0 (stale _output_get) 0.0) "1.000000,1.000000,0.700000") false false)
                (bind _output_get (Variables|Default|SetNow_R_arm_rotationY (+ (Variables|Default|GetNow_R_arm_rotationY) (Variables|Default|GetR_arm_rotationY)))))))
          (:then_1
            (if (not (> (Variables|Default|GetMax_L_arm_rotationY) (Variables|Default|GetNow_L_arm_rotationY)))
              (Transformation|SetRelativeTransform (Variables|Default|GetL_arm) (Math|Transform|MakeTransform "-265.000000,0.000000,-110.000000" (Math|Rotator|MakeRotator 0.0 (stale _output_get_2) 0.0) "1.000000,1.000000,0.700000") false false)
              (bind _output_get_2 (Variables|Default|SetNow_L_arm_rotationY (- (Variables|Default|GetNow_L_arm_rotationY) (Variables|Default|GetL_arm_rotationY)))))))
        (else
          (Variables|Default|SetNowLocation_Z (.z _returnvalue)) ; 上昇中のZの値を取得する
          (Variables|Default|SetNowLocation_Y (.y _returnvalue))
          (Variables|Default|SetNowLocation_X (.x _returnvalue)))))
    (:then_2
      (if (< (Variables|Default|GetMax_Time_float) 0.0)
        (if (not (Variables|Default|Gethit_Down))
          (Variables|Default|SetTime_Down true))))))

(event EventBeginPlay
  (bind _returnvalue (Transformation|GetActorLocation))
  ;[1 1 1] ゴール地点を取得する
  (Variables|Default|SetGoalLocation_Z (.z _returnvalue))
  (Variables|Default|SetGoalLocation_Y (.y _returnvalue))
  (Variables|Default|SetGoalLocation_X (.x _returnvalue))
  (bind _returnvalue_2 (Rendering|Material|CreateDynamicMaterialInstance (Variables|Default|GetfakeShadow) 0 "/Game/fakeShadow/MI_FakeShadow.MI_FakeShadow" "None" :!class /Script/Engine.PrimitiveComponent))
  (Variables|Default|SetShadowInstance _returnvalue_2))

(event Collision|EventActorBeginOverlap
  (params (OtherActor :type Actor%20Object%20Reference))
  ;[1 1 1] 物を取った後の行動
  (Utilities|FlowControl|Sequence
    (:then_0
      (if (Actor|ActorHasTag OtherActor (Variables|Default|GetKeihin_Tag))
        (Variables|Default|SetCrean_down false :!label _label) ; 下がる変数をfalseにかえる
        (Variables|Default|SetTime_Down false)
        (Variables|Default|Sethit_Down true)
        (Timeline|crean_arm_crose Play
          (:Update
            (Utilities|FlowControl|Sequence
              (:then_0
                (Transformation|SetRelativeTransform (Variables|Default|GetL_arm) (Math|Transform|MakeTransform (Math|Vector|MakeVector -265.0 0.0 -1.1e+02) (Math|Rotator|MakeRotator 0.0 (stale _output_get) 0.0) "1.000000,1.000000,0.700000") false false)
                (bind _output_get (Variables|Default|SetNow_L_arm_rotationY (+ (Variables|Default|GetNow_L_arm_rotationY) (Variables|Default|GetL_arm_rotationY)))))
              (:then_1
                (Transformation|SetRelativeTransform (Variables|Default|GetR_arm) (Math|Transform|MakeTransform (Math|Vector|MakeVector 2.7e+02 0.0 -1.1e+02) (Math|Rotator|MakeRotator 0.0 (stale _output_get_2) 0.0) "1.000000,1.000000,0.700000") false false)
                (bind _output_get_2 (Variables|Default|SetNow_R_arm_rotationY (- (Variables|Default|GetNow_R_arm_rotationY) (Variables|Default|GetR_arm_rotationY)))))))
          (:Finished
            (Utilities|FlowControl|Delay 2.0)
            (Timeline|Crean_TimeLine Play ; tickのようなもの
              (:Update
                (if (< (Variables|Default|GetGoalLocation_Z) (Variables|Default|GetNowLocation_Z)) ; Zの値がstartlineにいるかどうか
                  (if (< (Variables|Default|GetNowLocation_Y) (Variables|Default|GetGoalLocation_Y)) ; Yの値がstartlineにいるかどうか
                    (if (< (Variables|Default|GetNowLocation_X) (Variables|Default|GetGoalLocation_X)) ; Xの値がstartlineにいるかどうか
                      (Utilities|FlowControl|Sequence
                        (:then_0
                          (if (not (> (Variables|Default|GetNow_R_arm_rotationY) (Variables|Default|GetMax_R_arm_rotationY)))
                            (Transformation|SetRelativeTransform (Variables|Default|GetR_arm) (Math|Transform|MakeTransform "270.000000,0.000000,-110.000000" (Math|Rotator|MakeRotator 0.0 (stale _output_get_3) 0.0) "1.000000,1.000000,0.700000") false false)
                            (bind _output_get_3 (Variables|Default|SetNow_R_arm_rotationY (+ (Variables|Default|GetNow_R_arm_rotationY) (Variables|Default|GetR_arm_rotationY))))))
                        (:then_1
                          (if (not (> (Variables|Default|GetMax_L_arm_rotationY) (Variables|Default|GetNow_L_arm_rotationY)))
                            (Transformation|SetRelativeTransform (Variables|Default|GetL_arm) (Math|Transform|MakeTransform "-265.000000,0.000000,-110.000000" (Math|Rotator|MakeRotator 0.0 (stale _output_get_4) 0.0) "1.000000,1.000000,0.700000") false false)
                            (bind _output_get_4 (Variables|Default|SetNow_L_arm_rotationY (- (Variables|Default|GetNow_L_arm_rotationY) (Variables|Default|GetL_arm_rotationY)))))))
                      (else
                        (Transformation|SetActorTransform (Math|Transform|MakeTransform (+ (Transformation|GetWorldLocation (Variables|Default|GetBox)) (Variables|Default|Getcrean_offset_X) "") "0.000000,90.000000,0.000000")) ; Xの地点がstartラインに戻るまで移動
                      ))
                    (else
                      (Transformation|SetActorTransform (Math|Transform|MakeTransform (+ (Transformation|GetWorldLocation (Variables|Default|GetBox)) (Variables|Default|Getcrean_offset_Y) "") "0.000000,90.000000,0.000000")) ; Ｙの地点がstartラインに戻るまで移動
                    ))
                  (else
                    (Transformation|SetActorTransform (Math|Transform|MakeTransform (+ (Transformation|GetWorldLocation (Variables|Default|GetBox)) (Variables|Default|Getcrean_offset_Z) "") "0.000000,90.000000,0.000000")) ; Zの地点がstartラインに戻るまで移動
                  ))))))))
    (:then_1
      (if (Actor|ActorHasTag OtherActor (Variables|Default|GetFloor_Tag))
        (goto _label)))
    (:then_2
      ;[1 1 1] 壁に当たった場合の処理
      (if (Actor|ActorHasTag OtherActor (Variables|Default|GetWall_Tag))
        (Input|DisableInput 0)
        (Utilities|FlowControl|Sequence
          (:then_0
            (if (Actor|ActorHasTag OtherActor (Variables|Default|Gethaikei1_tag))
              (Transformation|SetActorTransform (Math|Transform|MakeTransform (+ (Transformation|GetWorldLocation (Variables|Default|GetBox)) (Variables|Default|Gethaikei1) "") "0.000000,90.000000,0.000000") true)
              (Input|EnableInput 0 :!label _label_2)))
          (:then_1
            (if (Actor|ActorHasTag OtherActor (Variables|Default|Gethaikei2_tag))
              (Transformation|SetActorTransform (Math|Transform|MakeTransform (+ (Transformation|GetWorldLocation (Variables|Default|GetBox)) (Variables|Default|Gethaikei2) "") "0.000000,90.000000,0.000000") true)
              (goto _label_2)))
          (:then_2
            (if (Actor|ActorHasTag OtherActor (Variables|Default|Getsokumen1_tag))
              (Transformation|SetActorTransform (Math|Transform|MakeTransform (+ (Transformation|GetWorldLocation (Variables|Default|GetBox)) (Variables|Default|Getsokumen1) "") "0.000000,90.000000,0.000000") true)
              (goto _label_2)))
          (:then_3
            (if (Actor|ActorHasTag OtherActor (Variables|Default|Getsokumen2_tag))
              (Transformation|SetActorTransform (Math|Transform|MakeTransform (+ (Transformation|GetWorldLocation (Variables|Default|GetBox)) (Variables|Default|Getsokumen2) "") "0.000000,90.000000,0.000000") true)
              (goto _label_2))))))))

(event Input|ActionEvents|InputActionshift
  (params (Key :type Key%20Structure :default "None"))
  ;[1 1 1] 下に動く
  (:Pressed
    (if (not (Variables|Default|GetBlockGrab))
      (Variables|Default|SetCrean_down true) ; 押されたかどうかの変数
      (Variables|Default|SetTime_Down true) ; 時間で処理される
    )))

(event Input|AxisEvents|InputAxismovefront
  (params (AxisValue :type Float%20%28single-precision%29))
  ;[1 1 1] 前後の動き
  (if (not (Variables|Default|GetCrean_down))
    (Pawn|Input|AddMovementInput (Math|Vector|GetForwardVector "0, 0, 0") AxisValue false)))

(event Input|AxisEvents|InputAxismoveright
  (params (AxisValue :type Float%20%28single-precision%29))
  ;[1 1 1] 左右の動き
  (if (not (Variables|Default|GetCrean_down))
    (Pawn|Input|AddMovementInput (Math|Vector|GetRightVector "0, 0, 0") AxisValue false)))

(fn ConstructionScript)